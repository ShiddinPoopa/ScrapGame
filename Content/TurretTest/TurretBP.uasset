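; Test turret Blueprint that rotates its Turret component to face the first-person character when it is within range.
; BeginPlay caches the character as Target, and Tick measures its distance to choose between AimAtTarget and ResetAim.
; Aiming converts the direction to the target into actor-local space and applies only pitch and yaw as relative rotation, without interpolation.
; ResetAim and FindTarget are empty stubs.
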(event Custom|AimAtTarget
  (bind _returnvalue (Transformation|GetActorTransform))
  (bind _turret (Variables|Default|GetTurret))
  (bind _targetlocation (Variables|Default|GetTargetLocation))
  (bind _returnvalue_2 (Transformation|GetWorldLocation _turret))
  (bind _returnvalue_3 (- _targetlocation _returnvalue_2))
  (bind _returnvalue_4 (Math|Transform|InverseTransformDirection _returnvalue _returnvalue_3))
  (bind _returnvalue_5 (Math|Rotator|MakeRotfromX _returnvalue_4))
  ;[1 1 1] Comment
  (Transformation|SetRelativeRotation (Variables|Default|GetTurret) (Math|Rotator|MakeRotator 0.0 (.pitch _returnvalue_5) (.yaw _returnvalue_5)) false false))

(event Custom|ResetAim)

(event EventBeginPlay
  ;[1 1 1] Comment
  (bind _returnvalue (Actor|GetActorOfClass "/Game/FirstPersonBP/Blueprints/FirstPersonCharacter.FirstPersonCharacter_C"))
  (Variables|Default|SetTarget _returnvalue))

(event EventTick
  (params (DeltaSeconds :type Float%20%28single-precision%29))
  ;[1 1 1] Comment
  (Variables|Default|SetTargetLocation (Transformation|GetActorLocation (Variables|Default|GetTarget)))
  ;[1 1 1] Comment
  (if (<= (Math|Vector|VectorLength (- (Transformation|GetActorLocation) (Variables|Default|GetTargetLocation))) 3e+03)
    (CallFunction|AimatTarget)
    (else
      (CallFunction|ResetAim))))

(fn ConstructionScript)

(fn FindTarget)