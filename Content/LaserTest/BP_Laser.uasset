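; BP_Laser is a beam weapon effect that fires from the first-person character's LaserDirection component.
; It attaches a Cascade beam emitter, and Shooting traces forward to set the beam's endpoints.
; Each shot spawns impact and sparks systems at the hit location, plus scorch and glow actor on blocking non-Enemy hits.
; Tick grows the range up to a cap while Firing, otherwise resets it, and matches beam visibility to Firing.
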(event Custom|Shooting
  (bind _fpref (Variables|Default|GetFPRef))
  (bind _laserdirection (Variables|/Game/FirstPersonBP/Blueprints/FirstPersonCharacter.FirstPersonCharacter_C|GetLaserDirection _fpref))
  (bind _returnvalue (Transformation|GetWorldLocation _laserdirection))
  ;[0 0.38 1] Spawn Emitter On player
  (Variables|Default|SetFiring true)
  (Utilities|FlowControl|Sequence
    (:then_0
      (Utilities|FlowControl|DoOnce false
        (:Completed
          (bind _returnvalue_2 (Effects|SpawnEmitterAttached "/Game/LaserTest/Laser_Cascade.Laser_Cascade" (Variables|/Game/FirstPersonBP/Blueprints/FirstPersonCharacter.FirstPersonCharacter_C|GetLaserDirection (Variables|Default|GetFPRef)) "None" "0, 0, 0" "0, 0, 0" "0.500000,0.500000,0.500000" "SnapToTarget" false))
          (Variables|Default|SetParticleRef _returnvalue_2))))
    (:then_1
      ;[0 1 0.2418] Set Laser Along Line
      (Class|ParticleSystemComponent|SetBeamSourcePoint (Variables|Default|GetParticleRef) 0 _returnvalue)
      (bind _outhit (Collision|LineTraceByChannel _returnvalue (+ _returnvalue (* (Math|Vector|GetForwardVector _laserdirection) (Variables|Default|GetRange))) "TraceTypeQuery1" false 0 "ForOneFrame"))
      ;[1 0.06761 0] Set End Point
      (Variables|Default|SetHit (.bblockinghit _outhit))
      (Variables|Default|SetHitLocation (.location _outhit))
      (Class|ParticleSystemComponent|SetBeamTargetPoint (Variables|Default|GetParticleRef) 0 (select (Variables|Default|GetHit) (Variables|Default|GetHitLocation) (.traceend _outhit)))
      ;[0 0.06638 1] Set Impact effects at hit location
      (Niagara|SpawnSystematLocation "/Game/LaserTest/LaserImpact_System.LaserImpact_System" (Variables|Default|GetHitLocation))
      (Niagara|SpawnSystematLocation "/Game/LaserTest/Sparks_System.Sparks_System" (Variables|Default|GetHitLocation) "0, 0, 0" "0.100000,0.100000,0.100000")
      (if (.bblockinghit _outhit)
        (if (not (Actor|ActorHasTag (.hitactor _outhit) "Enemy"))
          (Niagara|SpawnSystematLocation "/Game/LaserTest/Scroch_system.Scroch_system" (Variables|Default|GetHitLocation) "0, 0, 0" "0.100000,0.750000,0.750000")
          (Game|SpawnActorfromClass "/Game/LaserTest/LaserHitGlowBP.LaserHitGlowBP_C" (Math|Conversions|ToTransform(Vector) (Variables|Default|GetHitLocation)) "Undefined" 0 0))))))

(event EventBeginPlay
  ;[0 0.38 1] Spawn Emitter On player
  (bind _asfirst_person_character (Utilities|Casting|CastToFirstPersonCharacter (Game|GetPlayerCharacter 0)))
  (Variables|Default|SetFPRef _asfirst_person_character)
  (bind _returnvalue (Effects|SpawnEmitterAttached "/Game/LaserTest/Laser_Cascade.Laser_Cascade" (Variables|/Game/FirstPersonBP/Blueprints/FirstPersonCharacter.FirstPersonCharacter_C|GetLaserDirection (Variables|Default|GetFPRef)) "None" "0, 0, 0" "0, 0, 0" "0.500000,0.500000,0.500000" "SnapToTarget" false))
  (Variables|Default|SetParticleRef _returnvalue))

(event Collision|EventActorBeginOverlap
  (params (OtherActor :type Actor%20Object%20Reference)))

(event EventTick
  (params (DeltaSeconds :type Float%20%28single-precision%29))
  (bind _firing (Variables|Default|GetFiring))
  ;[1 0.0286 0] Set Visible
  (Rendering|SetVisibility (Variables|Default|GetParticleRef) _firing false)
  ;[0 1 0.0615] Extend Beam, set back when off
  (if _firing
    (if (and (< (Variables|Default|GetRange) 3e+03) (Variables|Default|GetFiring))
      (Variables|Default|SetRange (+ (Variables|Default|GetRange) (* DeltaSeconds 1e+03))))
    (else
      (Variables|Default|SetRange 0.0))))

(fn ConstructionScript)