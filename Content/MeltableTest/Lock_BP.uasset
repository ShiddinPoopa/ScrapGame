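; Lock_BP is a destructible lock that breaks when held under the laser.
; Each tick it finds the BP_Laser actor and drains Health while that laser's HitLocation is near the mesh origin, using a distance check rather than collision or damage events.
; When Health runs out, it spawns an effect system and a Lock_Debris_BP actor at the mesh location, then destroys itself.
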(event EventBeginPlay)

(event Collision|EventActorBeginOverlap
  (params (OtherActor :type Actor%20Object%20Reference)))

(event EventTick
  (params (DeltaSeconds :type Float%20%28single-precision%29))
  (bind _staticmesh (Variables|Default|GetStaticMesh))
  (bind _returnvalue (Transformation|GetWorldLocation _staticmesh))
  (bind _returnvalue_2 (Actor|GetActorOfClass "/Game/LaserTest/BP_Laser.BP_Laser_C"))
  (if (< (Math|Vector|Distance(Vector) (Transformation|GetWorldLocation (Variables|Default|GetStaticMesh)) (Variables|/Game/LaserTest/BP_Laser.BP_Laser_C|GetHitLocation _returnvalue_2)) 2e+01)
    (bind _output_get (Variables|Default|SetHealth (- (Variables|Default|GetHealth) 2.0)))
    (if (<= _output_get 0.0)
      (Niagara|SpawnSystematLocation 0 _returnvalue "0, 0, 0" "1.500000,1.500000,1.500000")
      (Variables|Default|SetDestroyed true)
      (if (Variables|Default|GetDestroyed)
        (Game|SpawnActorfromClass "/Game/MeltableTest/Lock_Debris_BP.Lock_Debris_BP_C" (Math|Conversions|ToTransform(Vector) _returnvalue) "Undefined" 0 0)
        (Actor|DestroyActor)))))

(fn ConstructionScript)